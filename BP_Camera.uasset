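; BP_Camera is a security camera that alerts guards when its AI perception spots the player.
; On each sensed perception update it sets CanSeePlayer, draws a debug box at the player and finds all BP_Guard actors.
; Guards sharing the camera's GroupID receive InvestigateCameraAlert with the player's current location and the camera's PatrolPoints.
; Losing sight only clears the flag; despite a "loop" comment, nothing repeats between perception updates.
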(event OnTargetPerceptionUpdated(AIPerception)
  (params (Actor :type Actor%20Object%20Reference) (Stimulus :type AI%20Stimulus%20Structure))
  (bind _returnvalue (Game|GetPlayerCharacter 0))
  (bind _capsulecomponent (Variables|/Script/Engine.Character|GetCapsuleComponent _returnvalue))
  (bind _returnvalue_2 (Transformation|GetWorldLocation _capsulecomponent))
  ;[1 1 1] Comment
  (Utilities|Casting|CastToBP_FirstPersonCharacter Actor)
  (if (.bSuccessfullySensed (Utilities|Struct|BreakAIStimulus Stimulus)) ; True if the player has just been spotted,\nFalse if the player has left our view.
    (Development|PrintString "Camera can see the player")
    (bind _output_get (Variables|Default|SetCanSeePlayer true))
    (if _output_get ; loop while you see the player
      (Rendering|Debug|DrawDebugBox :Center _returnvalue_2)
      (bind _outactors (Actor|GetAllActorsOfClass "/Game/BP_Guard.BP_Guard_C"))
      (for _array_element _outactors
        (if (== (Variables|Default|GetGroupID) (Variables|/Game/BP_Guard.BP_Guard_C|GetGroupID _array_element))
          (Development|PrintString "Sending Guards")
          (Default|InvestigateCameraAlert _array_element _returnvalue_2 (Variables|Default|GetPatrolPoints))))
      (else
        (Rendering|Debug|DrawDebugBox :Center _returnvalue_2)))
    (else
      (Development|PrintString "Camera can't see the player")
      (Variables|Default|SetCanSeePlayer false))))

(fn ConstructionScript)