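; BP_Guard is an AI guard that patrols, chases pawns it sees and catches the first-person player.
; A looping distance check on BeginPlay calls Caught on the player when within reach.
; PawnSensing triggers an AIMoveTo chase, then a walk through PatrolPointsGuard ending in a return to station.
; InvestigateCameraAlert sends the guard to an alerted location, then loops patrol over the points supplied with the alert.
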(event OnSeePawn(PawnSensing)
  (params (Pawn :type Pawn%20Object%20Reference))
  (Variables|Default|SetChasing true)
  (AI|AIMoveTo self (Transformation|GetActorLocation Pawn) Pawn 5e+01 false
    (:OnSuccess
      (Development|PrintString "We are at the player"))
    (:OnFail
      _))
  (Variables|Default|SetChasing false)
  (CallFunction|Patrol))

(event Custom|InvestigateCameraAlert
  (params (Destination :type Vector) (PatrolPoints :type Array%20of%20Actor%20Object%20References))
  (Rendering|Components|TextRender|SetText (Variables|Default|GetTextRender) (Utilities|Text|ToText(String) "Investigating"))
  (Development|PrintString "looking for player")
  (Variables|Default|SetPatrolling false)
  (Variables|Default|SetPatrolPoints PatrolPoints)
  (Variables|Default|SetIndex 0) ; Resets index (which patrol point we are looking at)
  (bind _movementresult (AI|AIMoveTo self Destination 0 1e+02 false)
    (:OnSuccess
      _)
    (:OnFail
      _))
  (switch Utilities|FlowControl|Switch|SwitchonEPathFollowingResult _movementresult
    (:Success
      (Development|PrintString "We are at the players last known location"))
    (:Blocked
      _)
    (:OffPath
      _)
    (:Invalid
      _))
  (Variables|Default|SetChasing false)
  (Utilities|FlowControl|Delay 1.0)
  (CallFunction|StartPatrol))

(event Custom|StartPatrol
  (Variables|Default|SetIndex 0) ; reset patrol index.
  (Variables|Default|SetPatrolling true)
  (Development|PrintString "now patrolling")
  (AI|AIMoveTo self (Transformation|GetActorLocation (Utilities|Array|Get(acopy) (Variables|Default|GetPatrolPoints) (Variables|Default|GetIndex))) 0 1e+02 false :!label _label
    (:OnSuccess
      _)
    (:OnFail
      _))
  (Utilities|FlowControl|Delay 2.0)
  (Math|Integer|IncrementInt (Variables|Default|GetIndex)
    (:%20%20
      (if (>= (Variables|Default|GetIndex) (Utilities|Array|Length (Variables|Default|GetPatrolPoints)))
        (CallFunction|StartPatrol)
        (elif (Variables|Default|GetPatrolling)
          (goto _label)
          (else
            (Development|PrintString "actively seeking the player now, cancelling patrol")))))))

(event Custom|Return%20to%20Guard%20Station
  (AI|AIMoveTo self (Variables|Default|GetStartLoc) 0 5.0 false))

(event Custom|Patrol
  (bind _index (Variables|Default|GetIndex))
  (AI|AIMoveTo self "0, 0, 0" (Utilities|Array|Get(acopy) (Variables|Default|GetPatrolPointsGuard) (Variables|Default|GetIndex)) 1e+02 false :!label _label
    (:OnSuccess
      _)
    (:OnFail
      _))
  (Utilities|FlowControl|Delay 0.2)
  (Math|Integer|IncrementInt _index
    (:%20%20
      (if (not (Variables|Default|GetChasing))
        (if (>= _index (Utilities|Array|Length (Variables|Default|GetPatrolPointsGuard)))
          (CallFunction|ReturntoGuardStation)
          (else
            (goto _label)))))))

(event EventBeginPlay
  (bind _capsulecomponent (Variables|Collision|GetCapsuleComponent))
  (bind _returnvalue (Transformation|GetWorldLocation _capsulecomponent))
  ;[1 1 1] Getting the player
  (Variables|Default|SetStartLocation _returnvalue)
  (Utilities|FlowControl|Delay 0.2 :!label _label)
  (if (<= (Math|Vector|Distance(Vector) _returnvalue (Transformation|GetWorldLocation (Variables|/Script/Engine.Character|GetCapsuleComponent (Game|GetPlayerCharacter 0)))) 1e+02)
    (Development|PrintString "Tag")
    (bind _asbp_first_person_character (Utilities|Casting|CastToBP_FirstPersonCharacter (Game|GetPlayerCharacter 0)))
    (Default|Caught _asbp_first_person_character)
    (goto _label)
    (else
      (goto _label))))

(fn ConstructionScript)